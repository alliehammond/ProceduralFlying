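; Actor component that handles player death by fading out and relocating its owner when the owner hits something.
; A hit creates and plays the FadingOut level sequence, with a flag blocking retriggers while it runs.
; A Tick timer then moves the owner to a random XY position at fixed height mid-sequence, and shortly after destroys the sequence actor and resets for the next hit.
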(event Custom|Actor%20Collided
  (params (SelfActor :type Actor%20Object%20Reference) (OtherActor :type Actor%20Object%20Reference) (NormalImpulse :type Vector) (Hit :type Hit%20Result%20Structure%20%28by%20ref%29))
  (if (not (Variables|Default|GetcreatedSequence))
    (Variables|Default|SetcreatedSequence true)
    (bind _outactor (Sequencer|Player|CreateLevelSequencePlayer "/Game/FadingOut.FadingOut"))
    (Sequencer|Player|Play (Variables|/Script/LevelSequence.LevelSequenceActor|GetSequencePlayer _outactor) :!class /Script/MovieScene.MovieSceneSequencePlayer)
    (Variables|Default|SetSeqPlayer _outactor)))

(event EventBeginPlay
  (Collision|BindEventtoOnActorHit (Components|GetOwner) (delegate Custom|Actor%20Collided)))

(event EventTick
  (params (DeltaSeconds :type Float%20%28single-precision%29))
  (if (Variables|Default|GetcreatedSequence)
    (bind _output_get (Variables|Default|SetplayerMoveTimer (+ DeltaSeconds (Variables|Default|GetplayerMoveTimer))))
    (if (> _output_get 1.4)
      (if (Variables|Default|GetplayedMoved)
        (if (> _output_get 2.2)
          (Variables|Default|SetcreatedSequence false)
          (Variables|Default|SetplayedMoved false)
          (Variables|Default|SetplayerMoveTimer 0.0)
          (Actor|DestroyActor (Variables|Default|GetSeqPlayer)))
        (else
          (Variables|Default|SetplayedMoved true)
          (Transformation|SetActorLocation (Components|GetOwner) (Math|Vector|MakeVector (Math|Random|RandomFloatinRange -5e+04 5e+04) (Math|Random|RandomFloatinRange -5e+04 5e+04) 3.5e+03) false false))))))